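; BP_Music is a level music actor that switches between ambiance and two combat intensity tracks as the first-person character enters trigger volumes.
; On BeginPlay it assigns the three tracks to their audio components and starts the ambiance.
; Switch1 hard-cuts from ambiance to intensity 1 on every player overlap, with no guard against retriggering.
; Switch2 cuts from intensity 1 to intensity 2, then clears the Box flag that gates it.
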(event OnComponentBeginOverlap(Switch1)
  (params (OverlappedComponent :type Primitive%20Component%20Object%20Reference) (OtherActor :type Actor%20Object%20Reference) (OtherComp :type Primitive%20Component%20Object%20Reference) (OtherBodyIndex :type Integer) (bFromSweep :type Boolean) (SweepResult :type Hit%20Result%20Structure%20%28by%20ref%29))
  (Utilities|Casting|CastToBP_FirstPersonCharacter OtherActor)
  (Audio|Components|Audio|Stop (Variables|Default|GetMusic_Ambiance))
  (Audio|Components|Audio|Play (Variables|Default|GetMusic_CombatIntensity1) 0.0))

(event OnComponentBeginOverlap(Switch2)
  (params (OverlappedComponent :type Primitive%20Component%20Object%20Reference) (OtherActor :type Actor%20Object%20Reference) (OtherComp :type Primitive%20Component%20Object%20Reference) (OtherBodyIndex :type Integer) (bFromSweep :type Boolean) (SweepResult :type Hit%20Result%20Structure%20%28by%20ref%29))
  (if (Variables|Default|GetBox)
    (Utilities|Casting|CastToBP_FirstPersonCharacter OtherActor)
    (Audio|Components|Audio|Stop (Variables|Default|GetMusic_CombatIntensity1))
    (Audio|Components|Audio|Play (Variables|Default|GetMusic_CombatIntensity2) 0.0)
    (Variables|Default|SetBox false)))

(event EventBeginPlay
  (bind _music_ambiance (Variables|Default|GetMusic_Ambiance))
  (Audio|Components|Audio|SetSound _music_ambiance "/Game/SFX/Musique/Music_Ambiance.Music_Ambiance")
  (Audio|Components|Audio|SetSound (Variables|Default|GetMusic_CombatIntensity1) "/Game/SFX/Musique/Music_CombatIntensity1.Music_CombatIntensity1")
  (Audio|Components|Audio|SetSound (Variables|Default|GetMusic_CombatIntensity2) "/Game/SFX/Musique/Music_CombatIntensity2.Music_CombatIntensity2")
  (Audio|Components|Audio|Play _music_ambiance 0.0))

(fn ConstructionScript)