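; Enemy projectile that flies a randomized curved path to TargetLocation and damages the first-person character on hit.
; At BeginPlay it offsets a random point along the line to the target sideways or vertically to form a control point.
; Each Tick the control point slides toward the target while the projectile chases it, bending the path without a spline.
; Any hit or arrival destroys mesh and collider, then the actor after a short delay.
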(event OnComponentHit(SphereCollider)
  (params (HitComponent :type Primitive%20Component%20Object%20Reference) (OtherActor :type Actor%20Object%20Reference) (OtherComp :type Primitive%20Component%20Object%20Reference) (NormalImpulse :type Vector :default "0, 0, 0") (Hit :type Hit%20Result%20Structure%20%28by%20ref%29))
  (bind _asbp_first_person_character (Utilities|Casting|CastToBP_FirstPersonCharacter OtherActor)
    (:then
      (Default|TakeDamage _asbp_first_person_character (Variables|Default|GetDamage)))
    (:CastFailed
      _))
  (Components|DestroyComponent (Variables|Default|GetProjectil%20Mesh))
  (Utilities|FlowControl|Delay 0.2)
  (Actor|DestroyActor))

(event EventBeginPlay
  (Utilities|FlowControl|Delay 0.01)
  (CallFunction|MidPointCalculator)
  (CallFunction|CurveControlPoint)
  (Components|Activation|Activate (Variables|Default|GetParticle%20Trail) false)
  (Utilities|FlowControl|Gate true) ; enters at Open
)

(event EventTick
  (params (DeltaSeconds :type Float%20%28single-precision%29))
  (Utilities|FlowControl|Gate true
    (:Exit
      (if (Utilities|Operators|NotEqual(!=) (Transformation|GetActorLocation) (Variables|Default|GetTargetLocation) 1e+01)
        (Variables|Default|SetCurved%20Point (Math|Interpolation|VInterptoConstant (Variables|Default|GetCurved%20Point) (Variables|Default|GetTargetLocation) (Utilities|Time|GetWorldDeltaSeconds) (Variables|Default|GetProjectile%20Speed)))
        (Transformation|SetActorLocation (Math|Interpolation|VInterptoConstant (Transformation|GetActorLocation) (Variables|Default|GetCurved%20Point) (Utilities|Time|GetWorldDeltaSeconds) (Variables|Default|GetProjectile%20Speed)) true false)
        (else
          (Components|DestroyComponent (Variables|Default|GetProjectil%20Mesh))
          (Utilities|FlowControl|Delay 0.2)
          (Actor|DestroyActor))))))

(fn ConstructionScript)

(fn MidPointCalculator
  (Variables|Default|SetMid%20Point (+ (* (- (Variables|Default|GetTargetLocation) (Transformation|GetActorLocation)) (Math|Random|RandomFloatinRange (Variables|Default|GetMin%20Curve%20Point%20Disctance) (Variables|Default|GetMax%20Curve%20Point%20Distance))) (Transformation|GetActorLocation))))

(fn CurveControlPoint
  (bind _mid_point (Variables|Default|GetMid%20Point))
  (bind _targetlocation (Variables|Default|GetTargetLocation))
  (bind _returnvalue (Math|Rotator|FindLookatRotation _mid_point _targetlocation))
  (bind (_x _y) (Math|Rotator|BreakRotIntoAxes _returnvalue))
  (Variables|Default|SetCurved%20Point (+ (Variables|Default|GetMid%20Point) (Math|Vector|RotateVectorAroundAxis (* (Math|Random|RandomFloatinRange (Variables|Default|GetMin%20Curve%20Radius) (Variables|Default|GetMax%20Curve%20Radius)) _y) 9e+01 _x))))

(fn RandomizeTargetLocation)