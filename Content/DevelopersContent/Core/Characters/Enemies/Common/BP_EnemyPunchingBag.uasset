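; BP_EnemyPunchingBag is an enemy that respawns in place after dying, serving as a reusable target.
; On death it spawns kill blood and a BP_Munition pickup, hides, then after RespawnTime reappears with full health and a refreshed life bar.
; Its construction script adds a Weapon box on the mesh's left-hand socket that overlaps only Pawns, and sizes the Range sphere from RangeSize.
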(event EventBeginPlay
  (|CallParentFunction))

(event EventDeath
  (params (Anim%20Index :type Integer))
  (bind _returnvalue (Transformation|GetActorLocation))
  (Niagara|SpawnSystematLocation "/Game/DevelopersContent/Core/Characters/Enemies/Common/Effects/NS_KillBlood.NS_KillBlood" _returnvalue)
  (Game|SpawnActorfromClass "/Game/NIRVANA/Core/Weapons/Common/BP_Munition.BP_Munition_C" (Math|Transform|MakeTransform _returnvalue "0, 0, 0" "1.000000,1.000000,1.000000") "Undefined" "MultiplyWithRoot" 0 "NewEnumerator5" 0)
  (Rendering|SetActorHiddenInGame true)
  (Utilities|FlowControl|Delay (Variables|Default|GetrespawnTime))
  (Rendering|SetActorHiddenInGame false)
  (Variables|Default|SetCurrentHealth (Variables|Default|GetMaxHealth))
  (CallFunction|SetLifeBar))

(fn ConstructionScript
  (|CallParentFunction)
  ;[1 1 1] cut
  (bind _returnvalue (AddComponent|AddBoxComponent true))
  (Variables|Default|SetWeapon _returnvalue)
  (bind _enumvalue (|ForEachECollisionChannel)
    (:LoopBody
      (Collision|SetCollisionResponsetoChannel (Variables|Default|GetWeapon) _enumvalue "ECR_Ignore"))
    (:then
      (Collision|SetCollisionResponsetoChannel (Variables|Default|GetWeapon) "ECC_Pawn" "ECR_Overlap")
      (Transformation|AttachComponentToComponent (Variables|Default|GetWeapon) (Variables|Character|GetMesh) "LeftHandSocket" "SnapToTarget" "SnapToTarget" "KeepRelative" true)
      (Components|Sphere|SetSphereRadius (Variables|Default|GetRange) (Variables|Default|GetRangeSize) true))))