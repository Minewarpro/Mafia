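; BP_AutoTurret is an automatic turret that shoots at the player while they are inside its Sphere1 overlap volume.
; Overlap events compare against a player reference cached on BeginPlay and toggle a Shoot flag.
; Fire re-triggers itself after a FireRate delay while Shoot is set.
; Each cycle turns the Sphere component toward the player in yaw only, then spawns a BP_BulletTurret at BulletSpawn after a short delay.
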(event OnComponentBeginOverlap(Sphere1)
  (params (OverlappedComponent :type Primitive%20Component%20Object%20Reference) (OtherActor :type Actor%20Object%20Reference) (OtherComp :type Primitive%20Component%20Object%20Reference) (OtherBodyIndex :type Integer) (bFromSweep :type Boolean) (SweepResult :type Hit%20Result%20Structure%20%28by%20ref%29))
  (if (== OtherActor (Variables|Default|Getplayerref))
    (Variables|Default|SetShoot true)
    (CallFunction|Fire)))

(event OnComponentEndOverlap(Sphere1)
  (params (OverlappedComponent :type Primitive%20Component%20Object%20Reference) (OtherActor :type Actor%20Object%20Reference) (OtherComp :type Primitive%20Component%20Object%20Reference) (OtherBodyIndex :type Integer))
  (if (== OtherActor (Variables|Default|Getplayerref))
    (Variables|Default|SetShoot false)))

(event Custom|Fire
  (if (Variables|Default|GetShoot)
    (Utilities|FlowControl|Sequence
      (:then_0
        (Transformation|SetWorldRotation (Variables|Default|GetSphere) (Math|Rotator|MakeRotator 0.0 0.0 (.yaw (Math|Interpolation|RInterpTo (Transformation|GetActorRotation) (Math|Rotator|FindLookatRotation (Transformation|GetActorLocation) (Transformation|GetActorLocation (Variables|Default|Getplayerref))) (Utilities|Time|GetWorldDeltaSeconds) (* 2e+01 5.0)))) false false))
      (:then_1
        (Utilities|FlowControl|Delay 0.1)
        (Game|SpawnActorfromClass "/Game/Blueprints/LevelDesign/BP_BulletTurret.BP_BulletTurret_C" (Transformation|GetWorldTransform (Variables|Default|GetBulletSpawn)) "Undefined" "MultiplyWithRoot" 0 0))
      (:then_2
        (if (Variables|Default|GetShoot)
          (Utilities|FlowControl|Delay (Variables|Default|GetFireRate))
          (CallFunction|Fire))))))

(event EventBeginPlay
  (bind _asbp_first_person_character (Utilities|Casting|CastToBP_FirstPersonCharacter (Game|GetPlayerCharacter 0)))
  (Variables|Default|Setplayerref _asbp_first_person_character))

(fn ConstructionScript)