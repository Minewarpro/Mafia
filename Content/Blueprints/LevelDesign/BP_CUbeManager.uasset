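; Level-design actor that builds a set of platform meshes and animates them between per-platform start and end locations.
; The construction script rebuilds them from a clamped Seed selecting manual, grid (optionally inclined) or circle (spiral or rise-and-fall) layouts.
; A single Timeline, rate-scaled by MovementSpeed, lerps every platform through MoveToEnd and MoveToStart.
; It can start on BeginPlay and, as a Repeater, ping-pongs after a wait.
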(event Custom|MoveToEnd
  (bind (_direction _alpha) (Timeline|Timeline Play)
    (:Update
      (for (_array_element _array_index) (Variables|Default|GetPlatforms)
        (Transformation|SetRelativeLocation _array_element (Math|Vector|Lerp(Vector) (.start (Utilities|Array|Get(acopy) (Variables|Default|GetLocations) _array_index)) (.end (Utilities|Array|Get(acopy) (Variables|Default|GetLocations) _array_index)) _alpha) false false)))
    (:Finished
      (if (Variables|Default|GetRepeater)
        (Utilities|FlowControl|Delay (Variables|Default|GetWaitingTime))
        (switch Utilities|FlowControl|Switch|SwitchonETimelineDirection _direction
          (:Forward
            (CallFunction|MovetoStart))
          (:Backward
            (CallFunction|MovetoEnd)))))))

(event Custom|MoveToStart
  (bind (_direction _alpha) (Timeline|Timeline Reverse)
    (:Update
      (for (_array_element _array_index) (Variables|Default|GetPlatforms)
        (Transformation|SetRelativeLocation _array_element (Math|Vector|Lerp(Vector) (.start (Utilities|Array|Get(acopy) (Variables|Default|GetLocations) _array_index)) (.end (Utilities|Array|Get(acopy) (Variables|Default|GetLocations) _array_index)) _alpha) false false)))
    (:Finished
      (if (Variables|Default|GetRepeater)
        (Utilities|FlowControl|Delay (Variables|Default|GetWaitingTime))
        (switch Utilities|FlowControl|Switch|SwitchonETimelineDirection _direction
          (:Forward
            (CallFunction|MovetoStart))
          (:Backward
            (CallFunction|MovetoEnd)))))))

(event EventBeginPlay
  (Components|Timeline|SetPlayRate (Variables|Default|GetTimeline) (/ 1.0 (Variables|Default|GetMovementSpeed)))
  (if (Variables|Default|GetActivatedDefault)
    (CallFunction|MovetoEnd)))

(fn ConstructionScript
  (CallFunction|CleanAll)
  (CallFunction|Reset)
  (if (< (Variables|Default|GetSeed) 0)
    (Variables|Default|SetSeed 0)
    (elif (> (Variables|Default|GetSeed) 2)
      (Variables|Default|SetSeed 2)))
  (switch int (Variables|Default|GetSeed)
    (:0
      (CallFunction|ManualMode))
    (:1
      (CallFunction|GenerateGrid))
    (:2
      (CallFunction|CirclePattern))))

(fn Reset
  (Utilities|Array|Clear (Variables|Default|GetLocations)))

(fn CleanAll
  (bind _platforms (Variables|Default|GetPlatforms))
  (for _array_element _platforms
    (Components|DestroyComponent _array_element))
  (Utilities|Array|Clear _platforms))

(fn AddMeshesonLocation
  (for _array_element (Variables|Default|GetLocations)
    (bind _returnvalue (AddComponent|AddStaticMeshComponent false (Math|Transform|MakeTransform (.start _array_element) "0, 0, 0" "1.000000,1.000000,1.000000")))
    (Components|StaticMesh|SetStaticMesh _returnvalue (Variables|Default|GetSMPlatform))
    (Utilities|Array|Add (Variables|Default|GetPlatforms) _returnvalue)))

(fn GenerateGrid
  (for _index (range 0 (- (Variables|Default|GetNbPlatformsX) 1))
    (Utilities|Array|Add (Variables|Default|GetLocations) (Utilities|Struct|MakeSPlatform (Math|Vector|MakeVector (* _index (Variables|Default|GetPlacementOffsetX)) 0.0 0.0) (Math|Vector|MakeVector (* _index (Variables|Default|GetPlacementOffsetX)) 0.0 (* _index (Variables|Default|GetOffsetHeight)))))
    (for _index_2 (range 0 (- (Variables|Default|GetNbPlatformsY) 1))
      (Utilities|Array|Add (Variables|Default|GetLocations) (Utilities|Struct|MakeSPlatform (Math|Vector|MakeVector (* _index (Variables|Default|GetPlacementOffsetX)) (* _index_2 (Variables|Default|GetPlacementOffsetY)) 0.0) (Math|Vector|MakeVector (* _index (Variables|Default|GetPlacementOffsetX)) (* _index_2 (Variables|Default|GetPlacementOffsetY)) (select (Variables|Default|GetInclined) (+ (* _index_2 (Variables|Default|GetOffsetHeight)) (* _index (Variables|Default|GetOffsetHeight))) (* _index (Variables|Default|GetOffsetHeight))))))))
  (CallFunction|AddMeshesonLocation))

(fn ManualMode
  (for _index (range 0 (- (Variables|Default|GetNbPlatformsX) 1))
    (Utilities|Array|Add :TargetArray (Variables|Default|GetLocations)))
  (CallFunction|AddMeshesonLocation))

(fn CirclePattern
  (bind _nbplatformsx (Variables|Default|GetNbPlatformsX))
  (for _index (range 0 _nbplatformsx)
    (Utilities|Array|Add (Variables|Default|GetLocations) (Utilities|Struct|MakeSPlatform (Math|Vector|MakeVector (.x (+ (* (Math|Vector|GetForwardVector (Math|Rotator|MakeRotator 0.0 0.0 (Math|Conversions|ToFloat(Integer) (* _index (/ 360 _nbplatformsx))))) (Variables|Default|GetRadiusMax)) (Variables|Default|GetCenterOfCircle))) (.y (+ (* (Math|Vector|GetForwardVector (Math|Rotator|MakeRotator 0.0 0.0 (Math|Conversions|ToFloat(Integer) (* _index (/ 360 _nbplatformsx))))) (Variables|Default|GetRadiusMax)) (Variables|Default|GetCenterOfCircle))) (.z (+ (* (Math|Vector|GetForwardVector (Math|Rotator|MakeRotator 0.0 0.0 (Math|Conversions|ToFloat(Integer) (* _index (/ 360 _nbplatformsx))))) (Variables|Default|GetRadiusMax)) (Variables|Default|GetCenterOfCircle)))) (Math|Vector|MakeVector (.x (+ (* (Math|Vector|GetForwardVector (Math|Rotator|MakeRotator 0.0 0.0 (Math|Conversions|ToFloat(Integer) (* _index (/ 360 _nbplatformsx))))) (Variables|Default|GetRadiusMax)) (Variables|Default|GetCenterOfCircle))) (.y (+ (* (Math|Vector|GetForwardVector (Math|Rotator|MakeRotator 0.0 0.0 (Math|Conversions|ToFloat(Integer) (* _index (/ 360 _nbplatformsx))))) (Variables|Default|GetRadiusMax)) (Variables|Default|GetCenterOfCircle))) (select (Variables|Default|GetSpiral) (+ (.z (+ (* (Math|Vector|GetForwardVector (Math|Rotator|MakeRotator 0.0 0.0 (Math|Conversions|ToFloat(Integer) (* _index (/ 360 _nbplatformsx))))) (Variables|Default|GetRadiusMax)) (Variables|Default|GetCenterOfCircle))) (* _index (Variables|Default|GetCircleHeigthDiff))) (select (<= _index (/ _nbplatformsx 2)) (+ (.z (+ (* (Math|Vector|GetForwardVector (Math|Rotator|MakeRotator 0.0 0.0 (Math|Conversions|ToFloat(Integer) (* _index (/ 360 _nbplatformsx))))) (Variables|Default|GetRadiusMax)) (Variables|Default|GetCenterOfCircle))) (* _index (Variables|Default|GetCircleHeigthDiff))) (+ (.z (+ (* (Math|Vector|GetForwardVector (Math|Rotator|MakeRotator 0.0 0.0 (Math|Conversions|ToFloat(Integer) (* _index (/ 360 _nbplatformsx))))) (Variables|Default|GetRadiusMax)) (Variables|Default|GetCenterOfCircle))) (* (- _nbplatformsx _index) (Variables|Default|GetCircleHeigthDiff)))))))))
  (CallFunction|AddMeshesonLocation))