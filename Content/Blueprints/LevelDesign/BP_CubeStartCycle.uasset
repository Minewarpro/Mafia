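; BP_CubeStartCycle is a one-shot level design trigger that starts movement on a set of arena actors when the player enters its box.
; BeginPlay caches the first-person player character so the overlap responds only to that actor.
; If Activated is set, the overlap clears it, then sets ActivatedDefault and calls MoveToEnd on every entry in ArenaToActivate.
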(event OnComponentBeginOverlap(Box)
  (params (OverlappedComponent :type Primitive%20Component%20Object%20Reference) (OtherActor :type Actor%20Object%20Reference) (OtherComp :type Primitive%20Component%20Object%20Reference) (OtherBodyIndex :type Integer) (bFromSweep :type Boolean) (SweepResult :type Hit%20Result%20Structure%20%28by%20ref%29))
  (if (== OtherActor (Variables|Default|GetPlayerRef))
    (if (Variables|Default|GetActivated)
      (Variables|Default|SetActivated false)
      (for _array_element (Variables|Default|GetArenaToActivate)
        (Variables|/Game/Blueprints/LevelDesign/BP_CUbeManager.BP_CUbeManager_C|SetActivatedDefault _array_element true)
        (Default|MovetoEnd _array_element)))))

(event EventBeginPlay
  (bind _asbp_first_person_character (Utilities|Casting|CastToBP_FirstPersonCharacter (Game|GetPlayerCharacter 0)))
  (Variables|Default|SetPlayerRef _asbp_first_person_character))

(fn ConstructionScript)