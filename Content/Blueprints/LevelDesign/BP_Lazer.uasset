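; BP_Lazer is a level-design laser actor that sizes its beam to the first blocking obstacle in front of it.
; On BeginPlay it caches the first-person character, then, if Active, runs one sphere trace along the Arrow's forward vector up to DetectorLength.
; The hit distance, or full detector length on a miss, becomes Laser1's Z scale.
; The trace runs only once and leaves persistent debug drawing.
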(event Custom|Laser
  (bind _arrow (Variables|Default|GetArrow))
  (bind _returnvalue (Transformation|GetWorldLocation _arrow))
  (if (Variables|Default|GetActive)
    (bind _outhit (Collision|SphereTraceByChannel _returnvalue (+ _returnvalue (* (Math|Vector|GetForwardVector _arrow) (Variables|Default|GetDetectorLength))) 25.0 "TraceTypeQuery1" false 0 "Persistent"))
    (if (.bblockinghit _outhit)
      (Variables|Default|SetLaserLength (/ (.distance _outhit) 1e+02))
      (CallFunction|Fire)
      (else
        (Variables|Default|SetLaserLength (/ (Variables|Default|GetDetectorLength) 1e+02))
        (CallFunction|Fire)))))

(event Custom|Fire
  (bind _laser1 (Variables|Default|GetLaser1))
  (bind _relativescale3d (Variables|/Script/Engine.SceneComponent|GetRelativeScale3D _laser1))
  (Transformation|SetRelativeScale3D _laser1 (Math|Vector|MakeVector (.x _relativescale3d) (.y _relativescale3d) (Variables|Default|GetLaserLength))))

(event EventBeginPlay
  (bind _asbp_first_person_character (Utilities|Casting|CastToBP_FirstPersonCharacter (Game|GetPlayerCharacter 0)))
  (Variables|Default|SetPlayerRef _asbp_first_person_character)
  (CallFunction|Laser))

(fn ConstructionScript)