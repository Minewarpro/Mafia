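; BP_HealthPack is a respawning health pickup that heals BP_FirstPersonCharacter on overlap.
; A timeline, rate-scaled at BeginPlay, spins the cube mesh in yaw and moves its relative height.
; On overlap, an active pack adds health only if the character is below max.
; It then hides itself and disables overlap events until a timer reactivates it after DesactivationTime.
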(event OnComponentBeginOverlap(BoxCollision)
  (params (OverlappedComponent :type Primitive%20Component%20Object%20Reference) (OtherActor :type Actor%20Object%20Reference) (OtherComp :type Primitive%20Component%20Object%20Reference) (OtherBodyIndex :type Integer) (bFromSweep :type Boolean) (SweepResult :type Hit%20Result%20Structure%20%28by%20ref%29))
  (bind _asbp_first_person_character (Utilities|Casting|CastToBP_FirstPersonCharacter OtherActor))
  (if (Variables|Default|GetIsActive)
    (if (< (Variables|/Game/FirstPerson/Blueprints/BP_FirstPersonCharacter.BP_FirstPersonCharacter_C|GetCurrent%20Health _asbp_first_person_character) (Variables|/Game/FirstPerson/Blueprints/BP_FirstPersonCharacter.BP_FirstPersonCharacter_C|GetMaxHealth _asbp_first_person_character))
      (Default|AddHealth _asbp_first_person_character (Variables|Default|GetHealth))
      (CallFunction|DesactivateHealth))))

(event Custom|Desactivate%20health
  (Variables|Default|SetIsActive false)
  (Utilities|Time|SetTimerbyEvent (delegate Custom|Activate%20Health) (Variables|Default|GetDesactivation%20Time))
  (Development|SetHiddeninGame (Variables|Default|GetCube) true false)
  (Variables|/Script/Engine.PrimitiveComponent|SetbGenerateOverlapEvents (Variables|Default|GetBox%20Collision) false))

(event Custom|Activate%20Health
  (Development|SetHiddeninGame (Variables|Default|GetCube) false false)
  (Variables|/Script/Engine.PrimitiveComponent|SetbGenerateOverlapEvents (Variables|Default|GetBox%20Collision) true)
  (Variables|Default|SetIsActive true))

(event EventBeginPlay
  (bind _cube (Variables|Default|GetCube))
  (Components|Timeline|SetPlayRate (Variables|Default|GetHealth%20Pack%20Turn_TL) (/ 1.0 3.0))
  (bind (_direction _rotation_alpha _z_location_alpha) (Timeline|Health%20Pack%20Turn_TL Play)
    (:Update
      (Transformation|SetRelativeRotation _cube (Math|Rotator|MakeRotator 0.0 0.0 (Math|Float|Lerp 0.0 3.6e+02 _rotation_alpha)) false false)
      (Transformation|SetRelativeLocation _cube (Math|Vector|MakeVector 0.0 0.0 (Math|Float|Lerp 575.0 6.5e+02 _z_location_alpha)) false false))))

(fn ConstructionScript)