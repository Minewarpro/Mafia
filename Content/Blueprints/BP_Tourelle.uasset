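; BP_Tourelle is a turret that repeatedly fires BP_EnemieProjectile shots from three muzzle points.
; On BeginPlay it caches the first-person player character, fires once immediately and starts a looping timer on ShootDelay.
; Each Shoot spawns one projectile per StartBullet component, passing that component's forward vector as Direction.
; It does no aiming, and the stored player reference is unused in these graphs.
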(event Custom|Shoot
  (bind _start_bullet2 (Variables|Default|GetStart%20Bullet2))
  (bind _start_bullet1 (Variables|Default|GetStart%20Bullet1))
  (bind _start_bullet (Variables|Default|GetStart%20Bullet))
  (Utilities|FlowControl|Sequence
    (:then_0
      (Game|SpawnActorfromClass "/Game/Blueprints/BP_EnemieProjectile.BP_EnemieProjectile_C" (Math|Transform|MakeTransform (Transformation|GetSocketLocation _start_bullet2 "None") "0, 0, 0" "1.000000,1.000000,1.000000") "Undefined" "SelectDefaultAtRuntime" 0 (Math|Vector|GetForwardVector _start_bullet2) 0))
    (:then_1
      (Game|SpawnActorfromClass "/Game/Blueprints/BP_EnemieProjectile.BP_EnemieProjectile_C" (Math|Transform|MakeTransform (Transformation|GetSocketLocation _start_bullet1 "None") "0, 0, 0" "1.000000,1.000000,1.000000") "Undefined" "SelectDefaultAtRuntime" 0 (Math|Vector|GetForwardVector _start_bullet1) 0))
    (:then_2
      (Game|SpawnActorfromClass "/Game/Blueprints/BP_EnemieProjectile.BP_EnemieProjectile_C" (Math|Transform|MakeTransform (Transformation|GetSocketLocation _start_bullet "None") "0, 0, 0" "1.000000,1.000000,1.000000") "Undefined" "SelectDefaultAtRuntime" 0 (Math|Vector|GetForwardVector _start_bullet) 0))))

(event EventBeginPlay
  (bind _asbp_first_person_character (Utilities|Casting|CastToBP_FirstPersonCharacter (Game|GetPlayerCharacter 0)))
  (Variables|Default|SetPlayerRef _asbp_first_person_character)
  (Utilities|Time|SetTimerbyEvent (delegate Custom|Shoot) (Variables|Default|GetShoot%20delay) true)
  (CallFunction|Shoot))

(fn ConstructionScript)