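; BP_Aspirable is an actor that the player's vacuum (aspirator) can suck in, through Aspired and StopAspired events.
; StopAspired stops the Aspir timeline, while Aspired is empty.
; Disconnected logic would play that timeline to lerp the actor from its stored location toward a target, then add aspirator munition to BP_FirstPersonCharacter and destroy the actor.
; As wired, that pull and pickup never runs.
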(event Custom|Aspired)

(event Custom|Stop%20Aspired
  (Audio|Components|Audio|Stop (Variables|Default|GetASpir)))

(fn ConstructionScript)