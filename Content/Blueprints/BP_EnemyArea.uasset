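; BP_EnemyArea is a box-shaped enemy zone that tracks how many NPCs it holds and spawns BP_EnemyRange enemies inside it.
; On BeginPlay a box trace claims enemies already inside, counts them and, after a short delay, clears their change-area flag.
; SpawnNPC places new enemies at random yaw-rotated points in the inner box, projected onto navigation.
; The point search retries recursively when projection lands near world origin.
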(event EventBeginPlay
  (bind _box (Variables|Default|GetBox))
  (bind _returnvalue (Transformation|GetWorldLocation _box))
  (bind _outhits (Class|KismetSystemLibrary|BoxTraceMulti _returnvalue _returnvalue (* (Variables|/Script/Engine.BoxComponent|GetBoxExtent _box) (Transformation|GetActorScale3D)) (Transformation|GetWorldRotation _box) "TraceTypeQuery3" false 0 "None" true))
  (bind _array_element (Utilities|Array|ForEachLoopwithBreak _outhits)
    (:LoopBody
      (bind _asbp_enemy_range (Utilities|Casting|CastToBP_EnemyRange (.hitactor _array_element)))
      (Variables|/Game/AI/BP_EnemyRange.BP_EnemyRange_C|SetArea _asbp_enemy_range self)
      (CallFunction|AddNPC 1)
      (Utilities|FlowControl|Delay 0.1)
      (Default|SetNeedChangeAreaValue _asbp_enemy_range false))))

(fn ConstructionScript
  (Components|Box|SetBoxExtent (Variables|Default|GetBox) (Variables|Default|GetIn%20Box%20Extent) true))

(fn SpawnNPC
  (params (Total%20Enemies :type Array%20of%20BP%20Enemy%20Range%20Object%20References))
  (bind _random_point (CallFunction|GetRandomPointinArea))
  (bind _returnvalue (Game|SpawnActorfromClass "/Game/AI/BP_EnemyRange.BP_EnemyRange_C" (Math|Transform|MakeTransform _random_point "0, 0, 0" "1.000000,1.000000,1.000000") "Undefined" "MultiplyWithRoot" 0 self 0))
  (CallFunction|AddNPC 1)
  (Utilities|Array|Add Total%20Enemies _returnvalue)
  (return _returnvalue))

(fn AddNPC
  (params (Nb :type Integer))
  (Variables|Default|SetNb%20NPCs (Math|Integer|SelectInt (+ (Variables|Default|GetNb%20NPCs) Nb) 0 (> (+ (Variables|Default|GetNb%20NPCs) Nb) 0)))
  (return))

(fn GetRandomPointinArea
  (bind _returnvalue (Transformation|GetActorScale3D))
  (bind _box (Variables|Default|GetBox))
  (bind _returnvalue_2 (Transformation|GetWorldLocation _box))
  (bind _boxextent (Variables|/Script/Engine.BoxComponent|GetBoxExtent _box))
  (bind _returnvalue_3 (* _boxextent _returnvalue))
  (bind _returnvalue_4 (* _returnvalue_3 0.7))
  (bind _returnvalue_5 (Math|Random|RandomPointinBoundingBox _returnvalue_2 _returnvalue_4))
  (bind _output_get (LocalVariables|SetImpact%20Point (.ProjectedLocation (AI|Navigation|ProjectPointtoNavigation (+ (* (Math|Vector|RotateVectorAroundAxis (Math|Vector|GetUnitDirection(Vector) _returnvalue_2 _returnvalue_5) (.yaw (Transformation|GetActorRotation)) "0.000000,0.000000,1.000000") (Math|Vector|Distance(Vector) _returnvalue_5 _returnvalue_2)) _returnvalue_2) 0 0 "1.000000,1.000000,300.000000"))))
  (if (Utilities|Operators|EqualEqual :A _output_get :ErrorTolerance 1e+02)
    (CallFunction|GetRandomPointinArea)
    (else
      (return (LocalVariables|GetImpact%20Point)))))