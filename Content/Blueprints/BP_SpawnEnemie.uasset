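; Arena volume that spawns BP_NPC enemies and sets their PlayerInArena blackboard flag as the player enters or leaves.
; BeginPlay box-traces for existing NPCs and starts a looping timer that prunes dead entries and spawns at random navmesh-projected points below a cap, in bursts when numbers run low.
; Spawning stops once all assigned Leaders are invalid.
; Spawn registration and GetSpawner's least-crowded-area logic are unwired.
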(event OnComponentBeginOverlap(Box)
  (params (OverlappedComponent :type Primitive%20Component%20Object%20Reference) (OtherActor :type Actor%20Object%20Reference) (OtherComp :type Primitive%20Component%20Object%20Reference) (OtherBodyIndex :type Integer) (bFromSweep :type Boolean) (SweepResult :type Hit%20Result%20Structure%20%28by%20ref%29))
  (bind _total_enemies (Variables|Default|GetTotal%20Enemies))
  ;[1 1 1] Player Detection
  (Utilities|Casting|CastToBP_FirstPersonCharacter OtherActor)
  (Variables|Default|SetPlayerIn true)
  (for (_array_element _array_index) _total_enemies
    (Utilities|IsValid _array_element
      (:Is%20Valid
        (AI|Components|Blackboard|SetValueasBool (AI|GetBlackboard _array_element) (Utilities|Name|MakeLiteralName "PlayerInArena") true))
      (:Is%20Not%20Valid
        (Utilities|Array|RemoveIndex _total_enemies _array_index)))))

(event OnComponentEndOverlap(Box)
  (params (OverlappedComponent :type Primitive%20Component%20Object%20Reference) (OtherActor :type Actor%20Object%20Reference) (OtherComp :type Primitive%20Component%20Object%20Reference) (OtherBodyIndex :type Integer))
  (bind _total_enemies (Variables|Default|GetTotal%20Enemies))
  ;[1 1 1] Player Detection
  (Utilities|Casting|CastToBP_FirstPersonCharacter OtherActor)
  (Variables|Default|SetPlayerIn false)
  (for (_array_element _array_index) _total_enemies
    (Utilities|IsValid _array_element
      (:Is%20Valid
        (AI|Components|Blackboard|SetValueasBool (AI|GetBlackboard _array_element) (Utilities|Name|MakeLiteralName "PlayerInArena") false))
      (:Is%20Not%20Valid
        (Utilities|Array|RemoveIndex _total_enemies _array_index)))))

(event Custom|Spawn%20Enemie
  (bind _areas (Variables|Default|GetAreas))
  (bind _area_index (CallFunction|GetSpawner _areas))
  (bind _returnvalue (Game|SpawnActorfromClass "/Game/AI/BP_NPC.BP_NPC_C" (Math|Transform|MakeTransform (Variables|Default|GetImpact%20Point) "0, 0, 0" "1.000000,1.000000,1.000000") "Undefined" "MultiplyWithRoot" 0 3e+03 "NewEnumerator1" 1e+01 "NewEnumerator1" (Utilities|Array|Get(acopy) _areas _area_index) 0)))

(event Custom|Spawn%20Loop
  (bind _returnvalue (Utilities|Time|SetTimerbyEvent (delegate Custom|Testing%20Spawn) 5.0 true))
  (Variables|Default|SetSpawnHandle _returnvalue))

(event Custom|Testing%20Spawn
  (bind _returnvalue (Transformation|GetActorScale3D))
  (bind _box (Variables|Default|GetBox))
  (bind _total_enemies (Variables|Default|GetTotal%20Enemies))
  (bind _returnvalue_2 (Transformation|GetWorldLocation _box))
  (bind _boxextent (Variables|/Script/Engine.BoxComponent|GetBoxExtent _box))
  (bind _returnvalue_3 (* _boxextent _returnvalue))
  (bind _returnvalue_4 (Math|Random|RandomPointinBoundingBox _returnvalue_2 _returnvalue_3))
  (bind _projectedlocation (AI|Navigation|ProjectPointtoNavigation _returnvalue_4 0 0 _returnvalue_3))
  (for (_array_element _array_index) _total_enemies
    (Utilities|IsValid _array_element
      (:Is%20Not%20Valid
        (Utilities|Array|RemoveIndex _total_enemies _array_index))))
  ;[0.5677 0.2215 0] No Leader
  (if (== (Utilities|Array|Length (Variables|Default|GetLeaders)) 0)
    (if (CallFunction|CanSpawn) :!label _label
      (if (<= (Utilities|Array|Length (Variables|Default|GetTotal%20Enemies)) (Variables|Default|GetNb%20Enemie%20Cas%20Urgence))
        (for _index (range 0 (Variables|Default|GetNb%20Spawn%20Enemie%20Urgence))
          (Variables|Default|SetImpact%20Point _projectedlocation)
          (if (Utilities|Operators|NotEqual(!=) :A _projectedlocation)
            (CallFunction|SpawnEnemie)
            (else
              (CallFunction|TestingSpawn))))
        (else
          (Variables|Default|SetImpact%20Point _projectedlocation)
          (if (Utilities|Operators|NotEqual(!=) :A _projectedlocation)
            (CallFunction|SpawnEnemie)
            (else
              (CallFunction|TestingSpawn))))))
    (else
      ;[1 0.4338 0.08854] Check Leader
      (Variables|Default|SetValidLeader false)
      (for _array_element_2 (Variables|Default|GetLeaders)
        (Variables|Default|SetValidLeader (or (Variables|Default|GetValidLeader) (Utilities|IsValid _array_element_2))))
      ;;[0.1827 1 0.152] Spawn Ended
      (if (Variables|Default|GetValidLeader)
        (goto _label)
        (else
          (Utilities|Time|ClearandInvalidateTimerbyHandle (Variables|Default|GetSpawnHandle)))))))

(event EventBeginPlay
  (bind _box (Variables|Default|GetBox))
  (bind _returnvalue (Transformation|GetWorldLocation _box))
  (CallFunction|SpawnLoop)
  (bind _outhits (Class|KismetSystemLibrary|BoxTraceMulti _returnvalue _returnvalue (* (Variables|/Script/Engine.BoxComponent|GetBoxExtent _box) (Transformation|GetActorScale3D)) (Transformation|GetWorldRotation _box) "TraceTypeQuery3" false 0 "Persistent" true))
  (bind _array_element (Utilities|Array|ForEachLoopwithBreak _outhits)
    (:LoopBody
      (bind _asbp_npc (Utilities|Casting|CastToBP_NPC (.hitactor _array_element)))
      (Utilities|Array|Add (Variables|Default|GetTotal%20Enemies) _asbp_npc))))

(fn ConstructionScript
  (Components|Box|SetBoxExtent (Variables|Default|GetBox) (Variables|Default|GetIn%20Box%20Extent) true))

(fn CanSpawn
  (return (< (Utilities|Array|Length (Variables|Default|GetTotal%20Enemies)) (Variables|Default|GetNb%20Max%20Enemie))))

(fn GetSpawner
  (params (Areas :type Array%20of%20BP%20Enemy%20Area%20Object%20References)))

(fn AssignNPCtoArea
  (params (NPC :type BP%20NPC%20Object%20Reference) (Area :type BP%20Enemy%20Area%20Object%20Reference)))