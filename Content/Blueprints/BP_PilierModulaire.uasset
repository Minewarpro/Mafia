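; Modular pillar actor that builds a stacked column of static meshes in the editor, with a configurable number of floors.
; The construction script resizes the per-floor struct array to NombreEtage and adds a mesh component for each entry, using its pillar variant, quarter-turn rotation and uniform scale.
; Each floor's height offset accumulates from the previous meshes' bounding box top times their scale.
; A U debug key prints the second floor's mesh height.
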(event EventBeginPlay)

(event Collision|EventActorBeginOverlap
  (params (OtherActor :type Actor%20Object%20Reference)))

(event EventTick
  (params (DeltaSeconds :type Float%20%28single-precision%29)))

(event Input|KeyboardEvents|DebugKeyU
  (params (Key :type Key%20Structure) (ActionValue :type Input%20Action%20Value%20Structure))
  (:Pressed
    (Development|PrintString (Utilities|String|ToString(Float) (.z (.max (StaticMesh|GetBoundingBox (Utilities|Select :Index (.mesh (Utilities|Array|Get(acopy) (Variables|Default|GetStruct_Pillar) 1)) :NewEnumerator0 "/Game/Environment/KIT/Pillar_A.Pillar_A" :NewEnumerator1 "/Game/Environment/KIT/Pillar_B.Pillar_B" :NewEnumerator2 "/Game/Environment/KIT/Pillar_C.Pillar_C" :NewEnumerator3 "/Game/Environment/KIT/Pillar_D.Pillar_D" :NewEnumerator4 "/Game/Environment/KIT/Pillar_E.Pillar_E" :NewEnumerator5 "/Game/Environment/KIT/Pillar_F.Pillar_F"))))))))

(fn ConstructionScript
  (bind _struct_pillar (Variables|Default|GetStruct_Pillar))
  (Utilities|Array|Resize _struct_pillar (Variables|Default|GetNombre%20Etage))
  (Variables|Default|SetHauteurNextPillar 0.0)
  (for (_array_element _array_index) _struct_pillar
    (if (> _array_index 0)
      (bind _output_get (Variables|Default|SetHauteurNextPillar (+ (Variables|Default|GetHauteurNextPillar) (* (.z (.max (StaticMesh|GetBoundingBox (Utilities|Select :Index (.mesh (Utilities|Array|Get(acopy) (Variables|Default|GetStruct_Pillar) (- _array_index 1))) :NewEnumerator0 "/Game/Environment/KIT/Pillar_A.Pillar_A" :NewEnumerator1 "/Game/Environment/KIT/Pillar_B.Pillar_B" :NewEnumerator2 "/Game/Environment/KIT/Pillar_C.Pillar_C" :NewEnumerator3 "/Game/Environment/KIT/Pillar_D.Pillar_D" :NewEnumerator4 "/Game/Environment/KIT/Pillar_E.Pillar_E" :NewEnumerator5 "/Game/Environment/KIT/Pillar_F.Pillar_F")))) (.scale (Utilities|Array|Get(acopy) (Variables|Default|GetStruct_Pillar) (- _array_index 1))))))))
    (bind _returnvalue (AddComponent|AddStaticMeshComponent false (Math|Transform|MakeTransform (Math|Vector|MakeVector 0.0 0.0 _output_get) (Math|Rotator|MakeRotator 0.0 0.0 (Utilities|Select :Index (.Rotation (Utilities|Struct|BreakStruct_Pillar _array_element)) :NewEnumerator0 0.0 :NewEnumerator1 9e+01 :NewEnumerator2 1.8e+02 :NewEnumerator3 2.7e+02)) (Math|Conversions|ToVector(Float) (.Scale (Utilities|Struct|BreakStruct_Pillar _array_element))))))
    (Components|StaticMesh|SetStaticMesh _returnvalue (Utilities|Select :Index (.Mesh (Utilities|Struct|BreakStruct_Pillar _array_element)) :NewEnumerator0 "/Game/Environment/KIT/Pillar_A.Pillar_A" :NewEnumerator1 "/Game/Environment/KIT/Pillar_B.Pillar_B" :NewEnumerator2 "/Game/Environment/KIT/Pillar_C.Pillar_C" :NewEnumerator3 "/Game/Environment/KIT/Pillar_D.Pillar_D" :NewEnumerator4 "/Game/Environment/KIT/Pillar_E.Pillar_E" :NewEnumerator5 "/Game/Environment/KIT/Pillar_F.Pillar_F"))))