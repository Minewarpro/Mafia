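; BP_Laser is a laser hazard that damages the first-person player character on overlapping its capsule.
; The construction script sets the Niagara beam's end to EndLocation, then moves, rotates and sizes the capsule to span the beam.
; The capsule sits at half of EndLocation, with look-at rotation pitched 90 degrees and half-height from half the beam length.
; It also prints EndLocation as a long-lasting debug string.
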(event OnComponentBeginOverlap(Capsule)
  (params (OverlappedComponent :type Primitive%20Component%20Object%20Reference) (OtherActor :type Actor%20Object%20Reference) (OtherComp :type Primitive%20Component%20Object%20Reference) (OtherBodyIndex :type Integer) (bFromSweep :type Boolean) (SweepResult :type Hit%20Result%20Structure%20%28by%20ref%29))
  (bind _asbp_first_person_character (Utilities|Casting|CastToBP_FirstPersonCharacter OtherActor))
  (Default|TakeDamage _asbp_first_person_character (Variables|Default|GetDamage)))

(fn ConstructionScript
  (bind _end_location (Variables|Default|GetEnd%20Location))
  (bind _ns_laserenemie (Variables|Default|GetNS_LaserEnemie))
  (bind _capsule (Variables|Default|GetCapsule))
  (bind _relativelocation (Variables|/Script/Engine.SceneComponent|GetRelativeLocation _ns_laserenemie))
  (bind _returnvalue (Math|Rotator|FindLookatRotation _relativelocation _end_location))
  (Development|PrintString (Utilities|String|ToString(Vector) (Variables|Default|GetEnd%20Location)) true true "(R=0.000000,G=0.660000,B=1.000000,A=1.000000)" 9e+10)
  (Niagara|SetNiagaraVariable(Vector3) (Variables|Default|GetNS_LaserEnemie) "Beam End" (Variables|Default|GetEnd%20Location))
  (Transformation|SetRelativeLocation _capsule (/ (Variables|Default|GetEnd%20Location) 2.0) false false)
  (Transformation|SetRelativeRotation _capsule (Math|Rotator|MakeRotator (.roll _returnvalue) (+ (.pitch _returnvalue) 9e+01) (.yaw _returnvalue)) false false)
  (Components|Capsule|SetCapsuleHalfHeight (Variables|Default|GetCapsule) (/ (Math|Vector|Distance(Vector) (Variables|/Script/Engine.SceneComponent|GetRelativeLocation (Variables|Default|GetNS_LaserEnemie)) (Variables|Default|GetEnd%20Location)) 2.0) true))