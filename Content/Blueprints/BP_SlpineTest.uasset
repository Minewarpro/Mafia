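; Test spline actor that tiles a mesh along its spline in the construction script, with no active runtime logic.
; It derives section length from the actor's Y scale and adds a collision-free spline mesh component, deformed along the Y axis, for each section.
; Each piece takes its endpoints and tangents from distances along the spline, with tangents clamped to section length.
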(event EventBeginPlay)

(event Collision|EventActorBeginOverlap
  (params (OtherActor :type Actor%20Object%20Reference)))

(event EventTick
  (params (DeltaSeconds :type Float%20%28single-precision%29)))

(fn ConstructionScript
  (bind _spline (Variables|Default|GetSpline))
  (bind _spline_2 (Variables|Default|GetSpline))
  (Variables|Default|Setsection%20lenght (* (.y (Transformation|GetActorScale3D)) 1e+02))
  (for _index (range 0 (Math|Float|Truncate (/ (Spline|GetSplineLength (Variables|Default|GetSpline)) (Variables|Default|Getsection%20lenght))))
    (bind _returnvalue (AddComponent|AddSplineMeshComponent false (Math|Transform|MakeTransform "0, 0, 0" "0, 0, 0" (Variables|Default|GetMesh%20Scale))))
    (Components|StaticMesh|SetStaticMesh _returnvalue (Variables|Default|GetMesh))
    (SplineMesh|SetForwardAxis _returnvalue "Y" true)
    (Collision|SetCollisionEnabled _returnvalue "NoCollision")
    (SplineMesh|SetStartandEnd _returnvalue (Spline|GetLocationatDistanceAlongSpline _spline_2 (* (Variables|Default|Getsection%20lenght) _index) "Local") (Math|Vector|ClampVectorSize (Spline|GetTangentatDistanceAlongSpline _spline_2 (* (Variables|Default|Getsection%20lenght) _index) "Local") 0.0 (Variables|Default|Getsection%20lenght)) (Spline|GetLocationatDistanceAlongSpline _spline (* (Variables|Default|Getsection%20lenght) (+ _index 1)) "Local") (Math|Vector|ClampVectorSize (Spline|GetTangentatDistanceAlongSpline _spline (* (Variables|Default|Getsection%20lenght) (+ _index 1)) "Local") 0.0 (Variables|Default|Getsection%20lenght)) true :!class /Script/Engine.SplineMeshComponent)))