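; BP_Spwan is a wave spawner that spawns BP_NPC enemies at its own location, starting on BeginPlay.
; Each StructWave entry supplies a delay and an enemy count, which drives a loop that spawns the whole wave at once.
; StartNextWave then increments CurrentNbWave and calls itself until the array is exhausted, so waves advance on timers alone, regardless of surviving enemies.
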(event Custom|Start%20Next%20Wave
  (Utilities|FlowControl|Delay (.timer (Utilities|Array|Get(acopy) (Variables|Default|GetStruct%20Wave) (Variables|Default|GetCurrent%20nb%20Wave))))
  (for _index (range 0 (- (.ennemy (Utilities|Array|Get(acopy) (Variables|Default|GetStruct%20Wave) (Variables|Default|GetCurrent%20nb%20Wave))) -1))
    (Game|SpawnActorfromClass "/Game/AI/BP_NPC.BP_NPC_C" (Math|Transform|MakeTransform (Transformation|GetActorLocation) "0, 0, 0" "1.000000,1.000000,1.000000") "Undefined" "MultiplyWithRoot" 0 0)
    (Development|PrintString "Spawn"))
  (bind _output_get (Variables|Default|SetCurrent%20nb%20Wave (+ (Variables|Default|GetCurrent%20nb%20Wave) 1)))
  (if (< _output_get (Utilities|Array|Length (Variables|Default|GetStruct%20Wave)))
    (CallFunction|StartNextWave)))

(event EventBeginPlay
  (CallFunction|StartNextWave))

(fn ConstructionScript)