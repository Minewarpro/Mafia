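; An automatic door Blueprint that opens when the first-person player enters a trigger box and closes when they leave.
; BeginPlay caches the player character, and the box's overlap events compare against it to play or reverse a shared Timeline.
; The Timeline curve, scaled by a NewHeight variable, drives the door component's relative Z location and prints that value each update.
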(event OnComponentBeginOverlap(Box)
  (params (OverlappedComponent :type Primitive%20Component%20Object%20Reference) (OtherActor :type Actor%20Object%20Reference) (OtherComp :type Primitive%20Component%20Object%20Reference) (OtherBodyIndex :type Integer) (bFromSweep :type Boolean) (SweepResult :type Hit%20Result%20Structure%20%28by%20ref%29))
  (if (== OtherActor (Variables|Default|GetPlayerRef))
    (CallFunction|OpenDoor)))

(event OnComponentEndOverlap(Box)
  (params (OverlappedComponent :type Primitive%20Component%20Object%20Reference) (OtherActor :type Actor%20Object%20Reference) (OtherComp :type Primitive%20Component%20Object%20Reference) (OtherBodyIndex :type Integer))
  (if (== OtherActor (Variables|Default|GetPlayerRef))
    (CallFunction|CloseDoor)))

(event Custom|OpenDoor
  (bind _newtrack_0 (Timeline|Timeline Play)
    (:Update
      (Development|PrintString (Utilities|String|ToString(Float) (* _newtrack_0 (Variables|Default|GetNewHeight))))
      (Transformation|SetRelativeLocation (Variables|Default|GetPorte) (Math|Vector|MakeVector 0.0 0.0 (* _newtrack_0 (Variables|Default|GetNewHeight))) false false))))

(event Custom|CloseDoor
  (bind _newtrack_0 (Timeline|Timeline Reverse)
    (:Update
      (Development|PrintString (Utilities|String|ToString(Float) (* _newtrack_0 (Variables|Default|GetNewHeight))))
      (Transformation|SetRelativeLocation (Variables|Default|GetPorte) (Math|Vector|MakeVector 0.0 0.0 (* _newtrack_0 (Variables|Default|GetNewHeight))) false false))))

(event EventBeginPlay
  (bind _asbp_first_person_character (Utilities|Casting|CastToBP_FirstPersonCharacter (Game|GetPlayerCharacter 0)))
  (Variables|Default|SetPlayerRef _asbp_first_person_character))

(fn ConstructionScript)