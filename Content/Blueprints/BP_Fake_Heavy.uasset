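; BP_Fake_Heavy is a turret-like enemy that tracks the first-person player and fires randomly chosen bullet patterns.
; A timeline eases the mesh toward the player, then a second keeps it locked on.
; Fire passes a valid pattern's settings to SpawnBullet, waits its post-delay and calls itself again.
; Hit reduces health and updates the widget life bar, or at zero spawns an explosion with sound and destroys the actor.
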(event Custom|Fire
  (bind _staticmesh (Variables|Default|GetStaticMesh))
  (bind _all_pattern (Variables|Default|GetAll%20Pattern))
  (Development|PrintString "Fire" true true "(R=1.000000,G=0.132552,B=0.000000,A=1.000000)")
  (Variables|Default|SetRandom%20Index (Math|Random|RandomInteger (Utilities|Array|Length _all_pattern)))
  (if (.isvalid (Utilities|Array|Get(acopy) _all_pattern (Variables|Default|GetRandom%20Index)))
    (Utilities|SpawnBullet (.pattern (Utilities|Array|Get(acopy) _all_pattern (Variables|Default|GetRandom%20Index))) (Transformation|GetWorldLocation _staticmesh) (Math|Vector|GetForwardVector _staticmesh) (.projectilespeed (Utilities|Array|Get(acopy) _all_pattern (Variables|Default|GetRandom%20Index))) (.damage (Utilities|Array|Get(acopy) _all_pattern (Variables|Default|GetRandom%20Index))) (.nbbulletloop (Utilities|Array|Get(acopy) _all_pattern (Variables|Default|GetRandom%20Index))) (.delayeachloop (Utilities|Array|Get(acopy) _all_pattern (Variables|Default|GetRandom%20Index))) (.dispertion (Utilities|Array|Get(acopy) _all_pattern (Variables|Default|GetRandom%20Index))) (.dispertionspeed (Utilities|Array|Get(acopy) _all_pattern (Variables|Default|GetRandom%20Index)))
      (:Out
        (Utilities|FlowControl|Delay (.delayafter (Utilities|Array|Get(acopy) _all_pattern (Variables|Default|GetRandom%20Index))))
        (Development|PrintString "End Delay")
        (CallFunction|Fire)))
    (else
      (CallFunction|Fire)
      (Development|PrintString "Not Valid"))))

(event Custom|Destroy
  (Game|SpawnActorfromClass "/Game/Blueprints/BP_ExplosionTurret.BP_ExplosionTurret_C" (Math|Transform|MakeTransform (Transformation|GetWorldLocation (Variables|Default|GetSphere)) "0, 0, 0" "1.000000,1.000000,1.000000") "Undefined" "MultiplyWithRoot" 0 0)
  (Audio|PlaySound2D "/Game/SFX/Explosion.Explosion" 1.0 1.0 0.0 0 0)
  (Actor|DestroyActor))

(event Custom|Start%20Target
  (bind _staticmesh (Variables|Default|GetStaticMesh))
  (Variables|Default|SetInit%20World%20Rotation (Transformation|GetWorldRotation _staticmesh))
  (bind _alpha_lerp (Timeline|Timeline_0 PlayFromStart)
    (:Update
      (Transformation|SetWorldRotation (Variables|Default|GetStaticMesh) (Math|Rotator|Lerp(Rotator) (Variables|Default|GetInit%20World%20Rotation) (Math|Rotator|FindLookatRotation (Transformation|GetWorldLocation _staticmesh) (Transformation|GetActorLocation (Variables|Default|GetPlayer%20Ref))) _alpha_lerp) false false))
    (:Finished
      (Timeline|Timeline Play
        (:Update
          (Transformation|SetWorldRotation (Variables|Default|GetStaticMesh) (Math|Rotator|FindLookatRotation (Transformation|GetWorldLocation (Variables|Default|GetStaticMesh)) (Transformation|GetActorLocation (Variables|Default|GetPlayer%20Ref))) false false))))))

(event EventBeginPlay
  (bind _asbp_first_person_character (Utilities|Casting|CastToBP_FirstPersonCharacter (Game|GetPlayerCharacter 0)))
  (Variables|Default|SetPlayer%20Ref _asbp_first_person_character)
  (CallFunction|StartTarget)
  (CallFunction|Fire)
  (Variables|Default|SetCurrent%20Health (Variables|Default|GetMax%20Health)))

(event EventHit
  (params (Damages :type Float%20%28double-precision%29))
  (bind _output_get (Variables|Default|SetCurrent%20Health (- (Variables|Default|GetCurrent%20Health) Damages)))
  (if (<= _output_get 0.0)
    (CallFunction|Destroy)
    (else
      (CallFunction|SetLifeBar))))

(fn ConstructionScript)

(fn SetLifeBar
  (bind _aswb_enemy_life_bar (Utilities|Casting|CastToWB_EnemyLifeBar (UserInterface|GetWidget (Variables|Default|GetWidget%20Life%20Bar))))
  (Default|SetProgressBar _aswb_enemy_life_bar (Math|Float|Clamp(Float) (/ (Variables|Default|GetCurrent%20Health) (Variables|Default|GetMax%20Health)))))