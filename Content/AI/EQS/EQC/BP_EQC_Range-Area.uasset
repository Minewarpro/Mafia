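; BP_EQC_Range-Area is an EQS context that provides a single location halfway between the querying enemy and an enemy area.
; For a BP_EnemyRange querier it uses that enemy's own Area reference.
; Any other querier falls back to GetActorOfClass for a BP_EnemyArea in the level.
; The midpoint comes from offsetting the querier's location by half the distance along the normalized direction to the area.
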(fn ProvideLocationsSet
  (params (QuerierObject :type Object%20Object%20Reference) (QuerierActor :type Actor%20Object%20Reference))
  (bind _returnvalue (Transformation|GetActorLocation QuerierActor))
  (bind _asbp_enemy_range (Utilities|Casting|CastToBP_EnemyRange QuerierActor)
    (:then
      (return (Utilities|Array|MakeArray (+ (Transformation|GetActorLocation _asbp_enemy_range) (* (Math|Vector|Normalize (- (Transformation|GetActorLocation (Variables|/Game/AI/Range/BP_EnemyRange.BP_EnemyRange_C|GetArea _asbp_enemy_range)) (Transformation|GetActorLocation _asbp_enemy_range))) (/ (Math|Vector|Distance(Vector) (Transformation|GetActorLocation (Variables|/Game/AI/Range/BP_EnemyRange.BP_EnemyRange_C|GetArea _asbp_enemy_range)) (Transformation|GetActorLocation _asbp_enemy_range)) 2.0))))))
    (:CastFailed
      (bind _returnvalue_2 (Actor|GetActorOfClass "/Game/Blueprints/LevelDesign/BP_EnemyArea.BP_EnemyArea_C"))
      (return (Utilities|Array|MakeArray (+ _returnvalue (* (Math|Vector|Normalize (- (Transformation|GetActorLocation _returnvalue_2) _returnvalue)) (/ (Math|Vector|Distance(Vector) (Transformation|GetActorLocation _returnvalue_2) _returnvalue) 2.0))))))))