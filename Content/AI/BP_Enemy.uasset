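; Enemy character Blueprint that takes damage, shows a life bar and can jump to a given destination.
; Hits update the bar and flash the player's crosshair through a timeline; death spawns blood VFX and a munition actor.
; Jumps launch on a montage notify using a suggested projectile arc adjusted for height difference.
; The IsJumping blackboard flag and zeroed walk speed coordinate takeoff and landing montages with AI.
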(event Custom|Death
  (params (Anim%20Index :type Integer))
  (bind _returnvalue (Transformation|GetActorLocation))
  ;[0.0226 0.0399 0.08854] Death
  (Niagara|SpawnSystematLocation "/Game/VFX/Enemies/NS_KillBlood.NS_KillBlood" _returnvalue)
  (Game|SpawnActorfromClass "/Game/Blueprints/BP_Munition.BP_Munition_C" (Math|Transform|MakeTransform _returnvalue "0, 0, 0" "1.000000,1.000000,1.000000") "Undefined" "MultiplyWithRoot" 0 0)
  (Actor|DestroyActor))

(event Custom|Cross%20hair%20hit%20alpha%20decrease
  ;[0.6667 0.6667 0.6667] Cross Widget
  (Variables|/Game/FirstPerson/Blueprints/BP_FirstPersonCharacter.BP_FirstPersonCharacter_C|SetCrosshair%20Hit%20Alpha (Variables|Default|GetPlayerRef) 1.0)
  (bind _alpha (Timeline|Timeline_0 PlayFromStart)
    (:Update
      (Variables|/Game/FirstPerson/Blueprints/BP_FirstPersonCharacter.BP_FirstPersonCharacter_C|SetCrosshair%20Hit%20Alpha (Variables|Default|GetPlayerRef) _alpha))))

(event EventBeginPlay
  ;[1 0.6945 0.125 1 34] Begin Play
  (bind _returnvalue (Actor|GetActorOfClass "/Game/FirstPerson/Blueprints/BP_FirstPersonCharacter.BP_FirstPersonCharacter_C"))
  (Variables|Default|SetPlayerRef _returnvalue)
  (Variables|HealthSystem|SetCurrentHealth (Variables|HealthSystem|GetMaxHealth)))

(event EventJumptoDestination
  (params (Destination :type Vector :default "0, 0, 0"))
  (bind _returnvalue (Transformation|GetActorLocation))
  (bind (_x _y _z) (Class|KismetMathLibrary|BreakVector3f Destination))
  (bind _charactermovement (Variables|Character|GetCharacterMovement))
  (bind _returnvalue_2 (- _returnvalue Destination))
  (bind _returnvalue_3 (< (.z _returnvalue_2) 0.0))
  (AI|Components|Blackboard|SetValueasBool (AI|GetBlackboard 0) (Utilities|Name|MakeLiteralName "IsJumping") true)
  (Variables|Default|SetTemp%20Max%20Walk%20Speed (Variables|/Script/Engine.CharacterMovementComponent|GetMaxWalkSpeed _charactermovement))
  (Variables|/Script/Engine.CharacterMovementComponent|SetMaxWalkSpeed _charactermovement 0.0)
  (bind _notifyname (Animation|Montage|PlayMontage (Variables|Character|GetMesh) "/Game/AI/Mixamo_Test/Anim/AM_Jumping_Start.AM_Jumping_Start")
    (:OnNotifyBegin
      (if (== _notifyname "JumpStart")
        (Variables|/Script/Engine.CharacterMovementComponent|SetMaxWalkSpeed (Variables|Character|GetCharacterMovement) (Variables|Default|GetTemp%20Max%20Walk%20Speed))
        (bind _outlaunchvelocity (Game|SuggestProjectileVelocityCustomArc _returnvalue (Math|Vector|MakeVector _x _y (+ _z 1.5e+02)) (Math|Float|SelectFloat (Components|Movement|GetGravityZ (Variables|Character|GetCharacterMovement)) 0.0 _returnvalue_3) 0.38))
        (Character|LaunchCharacter (* _outlaunchvelocity (Math|Float|SelectFloat 1.0 1.7 _returnvalue_3)) true true)))))

(event EventOnLanded
  (params (Hit :type Hit%20Result%20Structure%20%28by%20ref%29))
  (bind _charactermovement (Variables|Character|GetCharacterMovement))
  (Variables|Default|SetTemp%20Max%20Walk%20Speed (Variables|/Script/Engine.CharacterMovementComponent|GetMaxWalkSpeed _charactermovement))
  (Variables|/Script/Engine.CharacterMovementComponent|SetMaxWalkSpeed _charactermovement 0.0)
  (bind _notifyname (Animation|Montage|PlayMontage (Variables|Character|GetMesh) "/Game/AI/Mixamo_Test/Anim/AM_Falling_To_Landing.AM_Falling_To_Landing" 1.0 0.23)
    (:OnNotifyBegin
      (if (== _notifyname "CanWalk")
        (AI|Components|Blackboard|SetValueasBool (AI|GetBlackboard 0) (Utilities|Name|MakeLiteralName "IsJumping") false)
        (Variables|/Script/Engine.CharacterMovementComponent|SetMaxWalkSpeed (Variables|Character|GetCharacterMovement) (Variables|Default|GetTemp%20Max%20Walk%20Speed))))))

(event EventHit
  (params (Damages :type Float%20%28double-precision%29))
  ;[1 0.375 0.375] Hit
  (CallFunction|CrossHairHitAlphaDecrease)
  (Audio|PlaySound2D "/Game/SFX/Hit.Hit" 1.0 1.0 0.0 0 0)
  (bind _output_get (Variables|HealthSystem|SetCurrentHealth (- (Variables|HealthSystem|GetCurrentHealth) Damages)))
  (if (<= _output_get 0.0)
    (CallFunction|Death 2)
    (else
      (CallFunction|SetLifeBar))))

(fn ConstructionScript)

(fn SetLifeBar
  (bind _aswb_enemy_life_bar (Utilities|Casting|CastToWB_EnemyLifeBar (UserInterface|GetWidget (Variables|Default|GetWidgetLifeBar))))
  (Default|SetProgressBar _aswb_enemy_life_bar (Math|Float|Clamp(Float) (/ (Variables|HealthSystem|GetCurrentHealth) (Variables|HealthSystem|GetMaxHealth))))
  (return))