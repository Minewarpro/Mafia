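; Ranged enemy variant (V3) that randomizes its shot pattern on each Shoot before deferring to the parent's firing logic.
; A coin flip picks between two random-range pattern indices and one fixed index, converted to the Pattern enum.
; Cross and Hole Square patterns set DispertionSpeed faster when the player's DoomTest flag is on.
; On BeginPlay, TestingDoom enables a MaxHealth override, which is higher under DoomTest.
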(event EventBeginPlay
  (bind _playerref (Variables|Default|GetPlayerRef))
  (|CallParentFunction)
  (if (Variables|/Game/FirstPerson/Blueprints/BP_FirstPersonCharacter.BP_FirstPersonCharacter_C|GetTestingDoom _playerref)
    (Variables|Default|SetMaxHealth (Math|Float|SelectFloat 2e+03 5e+02 (Variables|/Game/FirstPerson/Blueprints/BP_FirstPersonCharacter.BP_FirstPersonCharacter_C|GetDoomTest _playerref)))))

(event EventShoot
  (bind _playerref (Variables|Default|GetPlayerRef))
  (bind _doomtest (Variables|/Game/FirstPerson/Blueprints/BP_FirstPersonCharacter.BP_FirstPersonCharacter_C|GetDoomTest _playerref))
  (bind _returnvalue (not _doomtest))
  (bind _output_get (Variables|Default|SetPattern (Utilities|Enum|ByteToEnumEnum_Pattern (Math|Conversions|ToByte(Integer) (Math|Integer|SelectInt (Math|Random|RandomIntegerinRange 3 4) 6 (Math|Random|RandomBool))))))
  (switch Utilities|FlowControl|Switch|SwitchonEnum_Pattern _output_get
    (:NewEnumerator1
      _)
    (:NewEnumerator0
      _)
    (:NewEnumerator9
      _)
    (:NewEnumerator3
      (if _returnvalue
        (Variables|Default|SetDispertion%20Speed 2.0)
        (else
          (Variables|Default|SetDispertion%20Speed 3.0))))
    (:NewEnumerator4
      (if _returnvalue
        (Variables|Default|SetDispertion%20Speed 2.0)
        (else
          (Variables|Default|SetDispertion%20Speed 3.0))))
    (:NewEnumerator5
      (if _returnvalue
        (Variables|Default|SetDispertion%20Speed 2.0)
        (else
          (Variables|Default|SetDispertion%20Speed 1e+01)))))
  (|CallParentFunction))

(fn ConstructionScript
  (|CallParentFunction))