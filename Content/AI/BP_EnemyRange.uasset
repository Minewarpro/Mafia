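; Ranged enemy that fires patterned bullets from its left hand socket at the player, re-enabling attack after a delay.
; When its area has neighbors, it creates an info widget and a looping timer moves it to a random next area, updating NPC counts and the blackboard target point.
; Range and capsule overlaps toggle blackboard flags for player proximity and area changes.
; On death it releases its token on the player.
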(event OnComponentBeginOverlap(Range)
  (params (OverlappedComponent :type Primitive%20Component%20Object%20Reference) (OtherActor :type Actor%20Object%20Reference) (OtherComp :type Primitive%20Component%20Object%20Reference) (OtherBodyIndex :type Integer) (bFromSweep :type Boolean) (SweepResult :type Hit%20Result%20Structure%20%28by%20ref%29))
  (bind _self self)
  (bind _returnvalue (AI|GetAIController _self))
  (bind _returnvalue_2 (AI|GetBlackboard _returnvalue))
  (Utilities|Casting|CastToBP_FirstPersonCharacter OtherActor)
  (AI|Components|Blackboard|SetValueasBool _returnvalue_2 (Utilities|Name|MakeLiteralName "PlayerInRange") true)
  (AI|Components|Blackboard|SetValueasBool _returnvalue_2 (Utilities|Name|MakeLiteralName "NeedChangeArea") false))

(event OnComponentEndOverlap(Range)
  (params (OverlappedComponent :type Primitive%20Component%20Object%20Reference) (OtherActor :type Actor%20Object%20Reference) (OtherComp :type Primitive%20Component%20Object%20Reference) (OtherBodyIndex :type Integer))
  (bind _self self)
  (bind _returnvalue (AI|GetAIController _self))
  (bind _returnvalue_2 (AI|GetBlackboard _returnvalue))
  (Utilities|Casting|CastToBP_FirstPersonCharacter OtherActor)
  (Utilities|IsValid _returnvalue_2
    (:Is%20Valid
      (AI|Components|Blackboard|SetValueasBool _returnvalue_2 (Utilities|Name|MakeLiteralName "PlayerInRange") false)
      (AI|Components|Blackboard|SetValueasBool _returnvalue_2 (Utilities|Name|MakeLiteralName "NeedChangeArea") true))))

(event OnComponentBeginOverlap(CapsuleComponent)
  (params (OverlappedComponent :type Primitive%20Component%20Object%20Reference) (OtherActor :type Actor%20Object%20Reference) (OtherComp :type Primitive%20Component%20Object%20Reference) (OtherBodyIndex :type Integer) (bFromSweep :type Boolean) (SweepResult :type Hit%20Result%20Structure%20%28by%20ref%29))
  (Utilities|Casting|CastToBP_EnemyArea OtherActor)
  (AI|Components|Blackboard|SetValueasBool (AI|GetBlackboard (AI|GetAIController self)) (Utilities|Name|MakeLiteralName "NeedChangeArea") false))

(event Custom|Shoot
  (bind _mesh (Variables|Character|GetMesh))
  (bind _returnvalue (Transformation|GetSocketLocation _mesh "LeftHandSocket"))
  ;[1 1 1] Shoot
  (Utilities|SpawnBullet (Variables|Default|GetPattern) _returnvalue (Math|Vector|GetUnitDirection(Vector) _returnvalue (Transformation|GetActorLocation (Variables|Default|GetPlayerRef))) 1.2e+03 (Variables|Default|GetDamage) (Variables|Default|GetNb%20Bullet%20/%20Loop) (Variables|Default|GetDelay%20Each%20Loop) (Variables|Default|GetPatternDispertion) (Variables|Default|GetDispertion%20Speed)
    (:Out
      (Utilities|FlowControl|Delay (Variables|Default|GetShootDelay))
      (Variables|Default|SetCanAttack true))))

(event Custom|Change%20Zone%20Loop
  ;[0.1367 0.2177 0.9375] Change Zone
  (bind _returnvalue (Utilities|Time|SetTimerbyEvent (delegate Custom|Changing%20Zone) 2.0 true))
  (Variables|Default|SetEventChangingZone _returnvalue))

(event Custom|Changing%20Zone
  ;[0.1367 0.2177 0.9375] Change Zone
  (Default|AddNPC (Variables|Default|GetArea) -1)
  (bind _output_get (Variables|Default|SetRandom%20Area (.OutItem (Utilities|Array|Random (Variables|/Game/Blueprints/LevelDesign/BP_EnemyArea.BP_EnemyArea_C|GetNext%20Areas (Variables|Default|GetArea))))))
  (Default|AddNPC _output_get 1)
  (Variables|Default|SetArea _output_get)
  (CallFunction|SetNeedChangeAreaValue true))

(event EventBeginPlay
  (|CallParentFunction)
  (if (> (Utilities|Array|Length (Variables|/Game/Blueprints/LevelDesign/BP_EnemyArea.BP_EnemyArea_C|GetNext%20Areas (Variables|Default|GetArea))) 0)
    (CallFunction|ChangeZoneLoop)
    (bind _returnvalue (UserInterface|CreateWidget "/Game/AI/WB_EnemyInfos.WB_EnemyInfos_C" 0 self))
    (Variables|Default|SetWidget%20infos _returnvalue)
    (UserInterface|SetWidget (Variables|Default|Getinfos) (Variables|Default|GetWidget%20infos))))

(event EventDeath
  (params (Anim%20Index :type Integer))
  (Default|ReleaseToken (Variables|Default|GetPlayerRef) (Variables|Default|GetToken)))

(fn ConstructionScript
  (|CallParentFunction))

(fn SetNeedChangeAreaValue
  (params (bool :type Boolean))
  (bind _returnvalue (AI|GetBlackboard 0))
  (bind _random_point (Default|GetRandomPointinArea (Variables|Default|GetArea)))
  (AI|Components|Blackboard|SetValueasVector _returnvalue (Utilities|Name|MakeLiteralName "TargetAreaLocation") _random_point)
  (AI|Components|Blackboard|SetValueasBool _returnvalue (Utilities|Name|MakeLiteralName "NeedChangeArea") bool)
  (return))