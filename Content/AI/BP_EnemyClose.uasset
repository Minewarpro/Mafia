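; BP_EnemyClose is a melee enemy that damages the first-person player when its weapon box overlaps them.
; Construction creates that Pawn-only box on the left-hand socket and sizes the Range sphere.
; A looping timer writes a navmesh-projected point just ahead of the player to the blackboard and prints an on-screen check.
; Range overlaps toggle the PlayerInRange key; BeginPlay starts with weapon overlaps disabled.
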(event OnComponentBeginOverlap(Range)
  (params (OverlappedComponent :type Primitive%20Component%20Object%20Reference) (OtherActor :type Actor%20Object%20Reference) (OtherComp :type Primitive%20Component%20Object%20Reference) (OtherBodyIndex :type Integer) (bFromSweep :type Boolean) (SweepResult :type Hit%20Result%20Structure%20%28by%20ref%29))
  ;[1 1 1] Range
  (Utilities|Casting|CastToBP_FirstPersonCharacter OtherActor)
  (AI|Components|Blackboard|SetValueasBool (AI|GetBlackboard 0) (Utilities|Name|MakeLiteralName "PlayerInRange") true))

(event OnComponentEndOverlap(Range)
  (params (OverlappedComponent :type Primitive%20Component%20Object%20Reference) (OtherActor :type Actor%20Object%20Reference) (OtherComp :type Primitive%20Component%20Object%20Reference) (OtherBodyIndex :type Integer))
  ;[1 1 1] Range
  (bind _asbp_first_person_character (Utilities|Casting|CastToBP_FirstPersonCharacter OtherActor))
  (Utilities|IsValid _asbp_first_person_character
    (:Is%20Valid
      (AI|Components|Blackboard|SetValueasBool (AI|GetBlackboard 0) (Utilities|Name|MakeLiteralName "PlayerInRange") false))))

(event OnComponentBeginOverlap(Weapon)
  (params (OverlappedComponent :type Primitive%20Component%20Object%20Reference) (OtherActor :type Actor%20Object%20Reference) (OtherComp :type Primitive%20Component%20Object%20Reference) (OtherBodyIndex :type Integer) (bFromSweep :type Boolean) (SweepResult :type Hit%20Result%20Structure%20%28by%20ref%29))
  ;[1 1 1] Hit Player (cut)
  (bind _asbp_first_person_character (Utilities|Casting|CastToBP_FirstPersonCharacter OtherActor))
  (Default|TakeDamage _asbp_first_person_character 1e+01))

(event Custom|GetPlayerLocation
  (bind _playerref (Variables|Default|GetPlayerRef))
  (AI|Components|Blackboard|SetValueasVector (AI|GetBlackboard 0) (Utilities|Name|MakeLiteralName "PlayerLocation") (.ProjectedLocation (AI|Navigation|ProjectPointtoNavigation (+ (Transformation|GetActorLocation _playerref) (* (Transformation|GetActorForwardVector _playerref) 15.0)) 0 0 "40.000000,40.000000,10000.000000")))
  (Development|PrintString (Utilities|String|ToString(Boolean) (CallFunction|IsonScreen 75.0))))

(event EventBeginPlay
  (|CallParentFunction)
  (Variables|/Script/Engine.PrimitiveComponent|SetbGenerateOverlapEvents (Variables|Default|GetWeapon) false)
  (Utilities|Time|SetTimerbyEvent (delegate Custom|GetPlayerLocation) 0.2 true))

(fn ConstructionScript
  (|CallParentFunction)
  ;[1 1 1] cut
  (bind _returnvalue (AddComponent|AddBoxComponent true))
  (Variables|Default|SetWeapon _returnvalue)
  (bind _enumvalue (|ForEachECollisionChannel)
    (:LoopBody
      (Collision|SetCollisionResponsetoChannel (Variables|Default|GetWeapon) _enumvalue "ECR_Ignore"))
    (:then
      (Collision|SetCollisionResponsetoChannel (Variables|Default|GetWeapon) "ECC_Pawn" "ECR_Overlap")
      (Transformation|AttachComponentToComponent (Variables|Default|GetWeapon) (Variables|Character|GetMesh) "LeftHandSocket" "SnapToTarget" "SnapToTarget" "KeepRelative" true)
      (Components|Sphere|SetSphereRadius (Variables|Default|GetRange) (Variables|Default|GetRangeSize) true))))