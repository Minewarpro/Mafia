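; BP_Laser is a laser beam hazard that damages the first-person player character on overlap.
; The Niagara beam stays hidden for a spawn delay, then appears stretched to EndLocation, and the actor destroys itself after its lifetime unless that is negative.
; SetCapsule fits the collision capsule along the beam by centring, rotating and sizing it from the beam origin and end point.
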(event OnComponentBeginOverlap(Capsule)
  (params (OverlappedComponent :type Primitive%20Component%20Object%20Reference) (OtherActor :type Actor%20Object%20Reference) (OtherComp :type Primitive%20Component%20Object%20Reference) (OtherBodyIndex :type Integer) (bFromSweep :type Boolean) (SweepResult :type Hit%20Result%20Structure%20%28by%20ref%29))
  (bind _asbp_first_person_character (Utilities|Casting|CastToBP_FirstPersonCharacter OtherActor))
  (Default|TakeDamage _asbp_first_person_character (Variables|Default|GetDamage)))

(event Custom|Destroy
  (Actor|DestroyActor))

(event EventBeginPlay
  (bind _laser_life_time_ (Variables|Default|GetLaser%20Life%20Time%20))
  (Niagara|SetNiagaraVariable(Vector3) (Variables|Default|GetNS_LaserEnemie) "Beam End" (Variables|Default|GetInit%20Location))
  (Rendering|SetVisibility (Variables|Default|GetNS_LaserEnemie) false false)
  (Utilities|FlowControl|Sequence
    (:then_0
      (if (not (< _laser_life_time_ 0.0))
        (Utilities|FlowControl|Delay (+ (Variables|Default|GetSpwn%20Delay) _laser_life_time_))
        (CallFunction|Destroy)))
    (:then_1
      (Utilities|FlowControl|Delay (Variables|Default|GetSpwn%20Delay))
      (Niagara|SetNiagaraVariable(Vector3) (Variables|Default|GetNS_LaserEnemie) "Beam End" (Variables|Default|GetEnd%20Location))
      (Rendering|SetVisibility (Variables|Default|GetNS_LaserEnemie) true false)
      (CallFunction|SetCapsule))))

(fn ConstructionScript)

(fn SetCapsule
  (bind _ns_laserenemie (Variables|Default|GetNS_LaserEnemie))
  (bind _end_location (Variables|Default|GetEnd%20Location))
  (bind _capsule (Variables|Default|GetCapsule))
  (bind _returnvalue (Transformation|GetWorldLocation _ns_laserenemie))
  (bind _returnvalue_2 (Math|Rotator|FindLookatRotation _returnvalue _end_location))
  (Transformation|SetRelativeLocation _capsule (/ (- (Variables|Default|GetEnd%20Location) (Transformation|GetWorldLocation (Variables|Default|GetNS_LaserEnemie))) 2.0) false false)
  (Transformation|SetRelativeRotation _capsule (Math|Rotator|MakeRotator (.roll _returnvalue_2) (+ (.pitch _returnvalue_2) 9e+01) (.yaw _returnvalue_2)) false false)
  (Components|Capsule|SetCapsuleHalfHeight (Variables|Default|GetCapsule) (/ (Math|Vector|Distance(Vector) (Transformation|GetWorldLocation (Variables|Default|GetNS_LaserEnemie)) (Variables|Default|GetEnd%20Location)) 2.0) true)
  (Components|Capsule|SetCapsuleRadius (Variables|Default|GetCapsule) 22.0 true))