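; BP_Bumper is a placeable gameplay bumper that launches the player character when it enters the bumper's box.
; On BeginPlay it caches player 0 as a BP_FirstPersonCharacter and ignores overlaps from any other actor.
; The launch takes X and Y velocity from bumper variables and scales the vertical velocity from the character's own JumpZVelocity by a factor.
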(event OnComponentBeginOverlap(Box)
  (params (OverlappedComponent :type Primitive%20Component%20Object%20Reference) (OtherActor :type Actor%20Object%20Reference) (OtherComp :type Primitive%20Component%20Object%20Reference) (OtherBodyIndex :type Integer) (bFromSweep :type Boolean) (SweepResult :type Hit%20Result%20Structure%20%28by%20ref%29))
  (bind _playerref (Variables|Default|GetPlayerRef))
  (if (== OtherActor (Variables|Default|GetPlayerRef))
    (Character|LaunchCharacter _playerref (Math|Vector|MakeVector (Variables|Default|GetXVelocity) (Variables|Default|GetYVelocity) (* (Variables|/Script/Engine.CharacterMovementComponent|GetJumpZVelocity (Variables|/Script/Engine.Character|GetCharacterMovement _playerref)) (Variables|Default|GetZVelocityFactor))) false false)))

(event EventBeginPlay
  (bind _asbp_first_person_character (Utilities|Casting|CastToBP_FirstPersonCharacter (Game|GetPlayerCharacter 0)))
  (Variables|Default|SetPlayerRef _asbp_first_person_character))

(fn ConstructionScript)