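; BP_EnemieProjectile is an enemy projectile that damages the player.
; On BeginPlay it launches its collision component by setting physics linear velocity from Direction and Speed, then caches the first-person player character.
; If NeedChangeDirection is set, it switches to a second direction and speed after a delay.
; Overlapping the player applies damage and destroys the projectile, as does any blocking hit, without damage.
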(event OnComponentBeginOverlap(Collision)
  (params (OverlappedComponent :type Primitive%20Component%20Object%20Reference) (OtherActor :type Actor%20Object%20Reference) (OtherComp :type Primitive%20Component%20Object%20Reference) (OtherBodyIndex :type Integer) (bFromSweep :type Boolean) (SweepResult :type Hit%20Result%20Structure%20%28by%20ref%29))
  (if (== OtherActor (Variables|Default|GetPlayer%20Ref))
    (Default|TakeDamage (Variables|Default|GetPlayer%20Ref) (Variables|Default|GetDamage))
    (Actor|DestroyActor)))

(event OnComponentHit(Collision)
  (params (HitComponent :type Primitive%20Component%20Object%20Reference) (OtherActor :type Actor%20Object%20Reference) (OtherComp :type Primitive%20Component%20Object%20Reference) (NormalImpulse :type Vector :default "0, 0, 0") (Hit :type Hit%20Result%20Structure%20%28by%20ref%29))
  (Actor|DestroyActor))

(event Custom|Change%20Velocity
  (Physics|SetPhysicsLinearVelocity (Variables|Default|GetCollision) (* (Variables|Default|GetNew%20Direction) (Variables|Default|GetNew%20Speed)) false "None"))

(event EventBeginPlay
  (Physics|SetPhysicsLinearVelocity (Variables|Default|GetCollision) (* (Variables|Default|GetDirection) (Variables|Default|GetSpeed)) false "None")
  (Utilities|FlowControl|Sequence
    (:then_0
      (bind _asbp_first_person_character (Utilities|Casting|CastToBP_FirstPersonCharacter (Game|GetPlayerCharacter 0)))
      (Variables|Default|SetPlayer%20Ref _asbp_first_person_character))
    (:then_1
      (if (Variables|Default|GetNeed%20Change%20Direction)
        (Utilities|FlowControl|Delay (Variables|Default|GetDelay%20Change%20DIrection))
        (CallFunction|ChangeVelocity)))))

(fn ConstructionScript)