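; Mid-range AI enemy variant, V3, that randomizes its shot pattern each time it fires.
; The Shoot override picks a Pattern enum value from a weighted random choice over a few fixed indices.
; It sets DispertionSpeed for the Simple Cross, Simple Cross 45 and Hole Square patterns, then hands firing to the parent Shoot.
; BeginPlay and construction only call the parent.
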(event EventBeginPlay
  (|CallParentFunction))

(event EventShoot
  (bind _output_get (Variables|Default|SetPattern (Utilities|Enum|ByteToEnumEnum_Pattern (Math|Conversions|ToByte(Integer) (Math|Integer|SelectInt (Math|Random|RandomIntegerinRange 3 4) 6 (Math|Random|RandomBool))))))
  (switch Utilities|FlowControl|Switch|SwitchonEnum_Pattern _output_get
    (:NewEnumerator1
      _)
    (:NewEnumerator0
      _)
    (:NewEnumerator9
      _)
    (:NewEnumerator3
      (Variables|Default|SetDispertion%20Speed 3.0))
    (:NewEnumerator4
      (Variables|Default|SetDispertion%20Speed 2.0))
    (:NewEnumerator5
      (Variables|Default|SetDispertion%20Speed 2.0)))
  (|CallParentFunction))

(fn ConstructionScript
  (|CallParentFunction))