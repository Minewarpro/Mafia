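; First-person chakram weapon that fires chakram projectiles on the shoot input, gated by munition and a shot cooldown.
; Each shot spawns a projectile at the Muzzle socket, aimed at a point set distance along the camera's forward vector from the character.
; A FlipFlop alternates the inverse-degree flag passed to each projectile, along with damage and a weapon reference.
; AddMunition clamps the count between zero and the maximum.
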(event Input|EnhancedActionEvents|EnhancedInputActionIA_Shoot
  (params (ActionValue :type Boolean) (ElapsedSeconds :type Float%20%28double-precision%29) (TriggeredSeconds :type Float%20%28double-precision%29) (InputAction :type Input%20Action%20Object%20Reference :default "/Game/NIRVANA/Core/Characters/FirstPerson/Input/Actions/IA_Shoot.IA_Shoot"))
  (bind _first_personcharacter (Variables|Default|GetFirst%20PersonCharacter))
  (bind _firstpersoncamera (Variables|/Game/NIRVANA/Core/Characters/FirstPerson/BP_FirstPersonCharacter.BP_FirstPersonCharacter_C|GetFirstPersonCamera _first_personcharacter))
  (bind _returnvalue (Transformation|GetWorldRotation _firstpersoncamera))
  (:Triggered
    (if (Variables|Default|GetCan%20Shot)
      (if (> (Variables|Default|GetCurrentMunition) 0)
        (bind _isa (Utilities|FlowControl|FlipFlop)
          (:A
            _)
          (:B
            _))
        (bind _output_get (Variables|Default|SetInverseDeg _isa))
        (Game|SpawnActorfromClass "/Game/NIRVANA/Core/Weapons/Chakram/BP_Chakram_Projectile.BP_Chakram_Projectile_C" (Math|Transform|MakeTransform (Transformation|GetSocketLocation "Muzzle") _returnvalue "1.000000,1.000000,1.000000") "AlwaysSpawn" "MultiplyWithRoot" 0 (+ (Transformation|GetActorLocation _first_personcharacter) (* (Math|Vector|GetForwardVector _returnvalue) (Variables|Default|GetDistance))) (Variables|Default|GetDamage) self _output_get _returnvalue 0)
        (CallFunction|AddMunition -1)
        (Variables|Default|SetCan%20Shot false)
        (Utilities|FlowControl|Delay (Variables|Default|Getdelay%20shoot))
        (Variables|Default|SetCan%20Shot true)))))

(event EventBeginPlay
  (|CallParentFunction) ; This node is disabled and will not be called.\nDrag off pins to build functionality.
)

(fn AddMunition
  (params (Add%20Munition :type Integer))
  (bind _maxmunition (Variables|Default|GetMaxMunition))
  (Variables|Default|SetCurrentMunition (+ Add%20Munition (Variables|Default|GetCurrentMunition)))
  (if (< (Variables|Default|GetCurrentMunition) 0)
    (Variables|Default|SetCurrentMunition 0)
    (elif (> (Variables|Default|GetCurrentMunition) _maxmunition)
      (Variables|Default|SetCurrentMunition _maxmunition))))